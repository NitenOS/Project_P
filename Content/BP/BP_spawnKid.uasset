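; BP_spawnKid is a trigger actor that moves the existing BP_followChild to a GoPoint when BP_testCharacter enters its box.
; BeginPlay finds the child; overlap sets its AsBeenSpawn flag and relocates it, and is ignored while that flag is set.
; Tick plays a Timeline while the flag is set, acting as a timer that clears the flag and resets itself when finished.
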(event `self.ReceiveBeginPlay`
  (bind _returnvalue (`GameplayStatics.GetActorOfClass` "/Game/BP/BP_followChild.BP_followChild_C"))
  (set `self.followChild` _returnvalue))

(event `self.ReceiveTick`
  (params (DeltaSeconds :type "Float (single-precision)"))
  (if (`/Game/BP/BP_followChild.asBeenSpawn` (`self.followChild`))
    (`Timeline|Timeline` :!label _label
      (:`Finished`
        (set `/Game/BP/BP_followChild.asBeenSpawn` false (`self.followChild`))
        (goto _label :!via `SetNewTime`)))))

(event `self.Box.OnComponentBeginOverlap`
  (params (OverlappedComponent :type "PrimitiveComponent Object Reference") (OtherActor :type "Actor Object Reference") (OtherComp :type "PrimitiveComponent Object Reference") (OtherBodyIndex :type Integer) (bFromSweep :type Boolean) (SweepResult :type "HitResult Structure (by ref)"))
  (bind _followchild (`self.followChild`))
  (if (not (`/Game/BP/BP_followChild.asBeenSpawn` (`self.followChild`)))
    (cast `/Game/BP/BP_testCharacter` OtherActor)
    (set `/Game/BP/BP_followChild.asBeenSpawn` true _followchild)
    (`self.K2_SetActorLocation` _followchild (`self.K2_GetActorLocation` (`self.goPoint`)) false false)))

(fn `UserConstructionScript`)