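; Test player character with focus zoom, door opening and hiding, plus input shortcuts that load the menu, game and end levels.
; Grab calls the open function on either door type returned by Grabing.
; In human form, holding Focus narrows the camera FOV via a reversible timeline.
; Human-form hiding adjusts stress BPM, disables gravity and interpolates the capsule into a BP_cachette spot, then back out on release.
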(event `InputAction|LVL END`
  (params (Key :type "Key Structure"))
  (:`Pressed`
    (`GameplayStatics.OpenLevelBySoftObjectPtr` "/Game/Level/LVL_EndGame.LVL_EndGame")))

(event `InputAction|LVL 2`
  (params (Key :type "Key Structure"))
  (:`Pressed`
    (`GameplayStatics.OpenLevelBySoftObjectPtr` "/Game/Level/LVL_mainNIGHTV2.LVL_mainNIGHTV2")))

(event `InputAction|LVL 1`
  (params (Key :type "Key Structure"))
  (:`Pressed`
    (`GameplayStatics.OpenLevelBySoftObjectPtr` "/Game/Level/LVL_mainGame.LVL_mainGame")))

(event `InputAction|LVL menu`
  (params (Key :type "Key Structure"))
  (:`Pressed`
    (`GameplayStatics.OpenLevelBySoftObjectPtr` "/Game/MenuStart.MenuStart")))

(event `self.ReceiveTick`
  (params (DeltaSeconds :type "Float (single-precision)")))

(event `InputAction|Focus`
  (params (Key :type "Key Structure"))
  (bind _humainform (`self.humainForm`))
  (:`Pressed`
    (if _humainform
      (bind (_direction _time) (`Timeline|Timeline_1` :!label _label)
        (:`Update`
          (`CameraComponent.SetFieldOfView` (`self.Camera`) (`KismetMathLibrary.Lerp` 90.0 45.0 _time))))))
  (:`Released`
    (if _humainform
      (goto _label :!via `Reverse`))))

(event `InputAction|Grab`
  (params (Key :type "Key Structure"))
  (:`Pressed`
    (bind _returnvalue (`self.Grabing`))
    (bind _asbp_porte (cast `/Game/Level/ASSET_Meuble/Maison/BP_Porte` _returnvalue)
      (:`then`
        (`/Game/Level/ASSET_Meuble/Maison/BP_Porte.J'ouvreLaPorte` _asbp_porte))
      (:`CastFailed`
        (bind _asbp_porte_avec_vitre (cast `/Game/Level/ASSET_Meuble/Maison/BP_PorteAvecVitre` _returnvalue))
        (`/Game/Level/ASSET_Meuble/Maison/BP_PorteAvecVitre.J'ouvreLaPorte` _asbp_porte_avec_vitre)))))

(event `InputAction|hide`
  (params (Key :type "Key Structure"))
  (:`Pressed`
    (if (`self.humainForm`)
      (bind _returnvalue (`self.hideChar` null))
      (bind _asbp_cachette (cast `/Game/BP/BP_cachette` _returnvalue))
      (bind _output_get (set `self.currentTable` _asbp_cachette))
      (bind _hidelocation (`/Game/BP/BP_cachette.hideIn` _output_get))
      (`self.changeBPM` false 25.0)
      (`KismetSystemLibrary.PrintString` (`KismetStringLibrary.Conv_DoubleToString` (`self.stressBPM`)))
      (set `CharacterMovementComponent.GravityScale` 0.0 (`self.CharacterMovement`))
      (bind (_direction _newtrack_3) (`Timeline|Timeline` :!via `PlayFromStart`)
        (:`Update`
          (`SceneComponent.K2_SetWorldLocation` (`self.CapsuleComponent`) (`KismetMathLibrary.VInterpTo` (`SceneComponent.K2_GetComponentLocation` (`self.CapsuleComponent`)) _hidelocation _newtrack_3 1.0) false false))
        (:`Finished`
          (`self.setIsHide` true)))))
  (:`Released`
    (if (`self.humainForm`)
      (bind _returnvalue_2 (`self.getIsHide`))
      (if _returnvalue_2
        (bind _unhidelocation (`/Game/BP/BP_cachette.hideOut` (`self.currentTable`)))
        (set `CharacterMovementComponent.GravityScale` 1.0 (`self.CharacterMovement`))
        (bind (_direction_2 _newtrack_3_2) (`Timeline|Timeline_0` :!via `PlayFromStart`)
          (:`Update`
            (`SceneComponent.K2_SetWorldLocation` (`self.CapsuleComponent`) (`KismetMathLibrary.VInterpTo` (`SceneComponent.K2_GetComponentLocation` (`self.CapsuleComponent`)) _unhidelocation _newtrack_3_2 1.0) false false))
          (:`Finished`
            (`self.setIsHide` false)))))))

(fn `UserConstructionScript`)