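; BP_Phone is a phone actor that plays two audio messages in sequence when the player character first enters its trigger box.
; An overlap by testCharacter sets a one-shot Check flag and starts Message1, whose finished event starts Message2.
; Message2 also starts immediately if Message1 is not playing after the play call.
; BeginPlay looks up a BP_PhoneCheck actor but leaves the result unused.
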(event `self.ReceiveBeginPlay`
  (`GameplayStatics.GetActorOfClass` "/Game/BP/BP_PhoneCheck.BP_PhoneCheck_C"))

(event `self.Box.OnComponentBeginOverlap`
  (params (OverlappedComponent :type "PrimitiveComponent Object Reference") (OtherActor :type "Actor Object Reference") (OtherComp :type "PrimitiveComponent Object Reference") (OtherBodyIndex :type Integer) (bFromSweep :type Boolean) (SweepResult :type "HitResult Structure (by ref)"))
  (bind _message1 (`self.message1`))
  (cast `testCharacter` OtherActor)
  (if (not (`self.check`))
    (set `self.check` true)
    (`AudioComponent.Play` _message1 0.0)
    (if (not (`AudioComponent.IsPlaying` _message1))
      (`AudioComponent.Play` (`self.message2`) 0.0))))

(event `self.message1.OnAudioFinished`
  (`AudioComponent.Play` (`self.message2`) 0.0))

(fn `UserConstructionScript`)