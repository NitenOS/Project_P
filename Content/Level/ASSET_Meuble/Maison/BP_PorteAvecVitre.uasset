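; BP_PorteAvecVitre is a house door with a glass pane that toggles between open and closed.
; A box trigger binds the toggle to BP_testCharacter's GOGRAB event while that character overlaps it, and opens a closed door automatically for BP_adoChild.
; The toggle snaps PorteCircle's relative rotation without animation and plays the matching open or close sound.
; AdoOuvertPorte is set on closing but never read here.
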(event `self.Box.OnComponentBeginOverlap`
  (params (OverlappedComponent :type "PrimitiveComponent Object Reference") (OtherActor :type "Actor Object Reference") (OtherComp :type "PrimitiveComponent Object Reference") (OtherBodyIndex :type Integer) (bFromSweep :type Boolean) (SweepResult :type "HitResult Structure (by ref)"))
  (cast `/Game/BP/BP_adoChild` OtherActor
    (:`then`
      (if (not (`self.J'ouvre la porte`))
        (`self.J'ouvreLaPorte`)
        (set `self.J'ouvre la porte` true)))
    (:`CastFailed`
      (bind _asbp_test_character (cast `/Game/BP/BP_testCharacter` OtherActor))
      (add `/Game/BP/BP_testCharacter.GOGRAB` _asbp_test_character (delegate `J'ouvreLaPorte`)))))

(event `J'ouvreLaPorte`
  (bind _audio (`self.Audio`))
  (bind _audio_2 (`self.Audio`))
  (if (`self.J'ouvre la porte`)
    (`SceneComponent.K2_SetRelativeRotation` :`self` (`self.Porte_Circle`))
    (set `self.J'ouvre la porte` false)
    (set `self.adoOuvertPorte` true)
    (`AudioComponent.SetSound` _audio (`self.Close`))
    (`AudioComponent.Play` _audio 0.0)
    (else
      (`SceneComponent.K2_SetRelativeRotation` (`self.Porte_Circle`) (struct :`Yaw` -80.0) false false)
      (set `self.J'ouvre la porte` true)
      (`AudioComponent.SetSound` _audio_2 (`self.Open`))
      (`AudioComponent.Play` _audio_2 0.0))))

(event `self.Box.OnComponentEndOverlap`
  (params (OverlappedComponent :type "PrimitiveComponent Object Reference") (OtherActor :type "Actor Object Reference") (OtherComp :type "PrimitiveComponent Object Reference") (OtherBodyIndex :type Integer))
  (bind _asbp_test_character (cast `/Game/BP/BP_testCharacter` OtherActor))
  (remove `/Game/BP/BP_testCharacter.GOGRAB` _asbp_test_character (delegate `J'ouvreLaPorte`)))

(fn `UserConstructionScript`)